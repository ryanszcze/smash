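; Projectile actor that flies without gravity at a low initial speed and adds to the Healthperc of an Astrid character it touches.
; The construction script configures the ProjectileMovement component.
; Tick runs a debug-drawn sphere trace at the actor's location, casts the hit actor to Astrid, and applies the increase through a DoOnce.
; The component hit event is empty and the projectile is never destroyed here.
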(event `self.ReceiveTick`
  (params (DeltaSeconds :type "Float (single-precision)"))
  (bind _returnvalue (`self.K2_GetActorLocation`))
  (bind _outhit (`KismetSystemLibrary.SphereTraceSingle` :`Start` _returnvalue :`End` _returnvalue :`Radius` 50.0 :`TraceChannel` "TraceTypeQuery1" :`DrawDebugType` "ForOneFrame"))
  (bind _asastrid (cast `/Game/Blueprints/Astrid` (`.HitActor` (`GameplayStatics.BreakHitResult` _outhit))))
  (`/Engine/EditorBlueprintResources/StandardMacros.DoOnce` false
    (:`Completed`
      (set `/Game/Blueprints/Astrid.healthperc` (+ (`/Game/Blueprints/Astrid.healthperc` _asastrid) 10.0) _asastrid))))

(event `self.StaticMesh.OnComponentHit`
  (params (HitComponent :type "PrimitiveComponent Object Reference") (OtherActor :type "Actor Object Reference") (OtherComp :type "PrimitiveComponent Object Reference") (NormalImpulse :type "Vector Structure") (Hit :type "HitResult Structure (by ref)")))

(fn `UserConstructionScript`
  (bind _projectilemovement (`self.ProjectileMovement`))
  (set `ProjectileMovementComponent.ProjectileGravityScale` 0.0 _projectilemovement)
  (set `ProjectileMovementComponent.InitialSpeed` 200.0 _projectilemovement))