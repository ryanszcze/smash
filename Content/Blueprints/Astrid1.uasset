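; Astrid is a playable Paper2D platform-fighter character with running, jumping, melee, projectile and once-per-airtime dash moves.
; Tick picks flipbooks from a State enum and idle/jump flags, turning the controller to face horizontal velocity.
; Melee and special play timed flipbooks before spawning attack actors, while the air dash briefly zeroes gravity.
; Damage accumulates in Healthperc and launches Astrid with the causer's velocity; K and L are hard-wired hit and destroy keys.
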(event `Key|K`
  (params (Key :type "Key Structure"))
  (:`Pressed`
    (set `self.SwapMe` true)))

(event `Key|K`
  (params (Key :type "Key Structure"))
  (:`Pressed`
    (set `self.healthperc` (+ (`self.healthperc`) 1.0))
    (set `self.isIdle` false)
    (set `self.State` "NewEnumerator4")
    (`KismetSystemLibrary.Delay` 3.0)))

(event `Key|Period`
  (params (Key :type "Key Structure"))
  (:`Pressed`
    (`Controller.SetIgnoreMoveInput` (`self.GetController`) true :!label _label)
    (set `self.isIdle` false)
    (`PaperFlipbookComponent.SetFlipbook` (`self.Sprite`) "/Game/2DSideScroller/Sprites/Astrid/Astrid_DSpecial/sprite.sprite")
    (`Controller.ResetIgnoreMoveInput` (`self.GetController`))))

(event `Spawn`
  (goto _label))

(event `Key|K`
  (params (Key :type "Key Structure"))
  (:`Pressed`
    (goto _label)))

(event `InputAction|Melee`
  (params (Key :type "Key Structure"))
  (:`Pressed`
    (set `self.isIdle` false)
    (if (not (`self.isJumping`))
      (set `MovementComponent.Velocity` (0.0 0.0 0.0) (`self.CharacterMovement`))
      (`Controller.SetIgnoreMoveInput` (`self.GetController`) true)
      (`PaperFlipbookComponent.SetFlipbook` (`self.Sprite`) "/Game/2DSideScroller/Sprites/Astrid/Astrid_FTilt/AstridFTilt12.AstridFTilt12")
      (`KismetSystemLibrary.Delay` 0.4)
      (`|SpawnActorFromClass` "/Game/Blueprints/Melee.Melee_C" (`SceneComponent.K2_GetComponentToWorld` (`self.Arrow1`)) "Undefined" "OverrideRootScale" null null)
      (`|SpawnActorFromClass` "/Game/Blueprints/Melee.Melee_C" (`SceneComponent.K2_GetComponentToWorld` (`self.Arrow2`)) "Undefined" "OverrideRootScale" null null)
      (`KismetSystemLibrary.Delay` 0.2)
      (set `self.isIdle` true)
      (`Controller.ResetIgnoreMoveInput` (`self.GetController`)))))

(event `self.ReceiveBeginPlay`)

(event `self.ReceiveTick`
  (params (DeltaSeconds :type "Float (single-precision)"))
  (`self.UpdateAnimation1`))

(event `self.OnLanded`
  (params (Hit :type "HitResult Structure (by ref)"))
  (set `self.canAirDash` true)
  (set `self.State` "NewEnumerator0")
  (set `self.isIdle` true)
  (set `self.isJumping` false))

(event `InputAction|Jump`
  (params (Key :type "Key Structure"))
  ;[1 1 1] General Animations
  (:`Pressed`
    (set `self.isJumping` true)
    (set `self.isIdle` false)
    (if (not (`self.isDashing`)) :!label _label_2
      (`self.Jump`)
      (`PaperFlipbookComponent.SetFlipbook` (`self.Sprite`) "/Game/2DSideScroller/Sprites/Astrid/Astrid_Jump/Astrid_Jumping.Astrid_Jumping")))
  (:`Released`
    (set `self.isJumping` true)
    (set `self.isIdle` false)
    (if (not (`self.isDashing`)) :!label _label_3
      (`self.StopJumping`)
      (set `self.State` "NewEnumerator0"))))

(event `UpdateAnimation1`
  (bind _returnvalue_x (`KismetMathLibrary.BreakVector` (`self.GetVelocity`)))
  (bind _returnvalue_x_2 (`KismetMathLibrary.BreakVector` (`self.GetVelocity`)))
  ;[1 1 1] General Animations
  (if (`self.isIdle`)
    (`PaperFlipbookComponent.SetFlipbook` (`self.Sprite`) (select `bool` (> (`KismetMathLibrary.VSize` (`KismetMathLibrary.Conv_DoubleToVector` _returnvalue_x_2)) 0.0) :`false` "/Game/2DSideScroller/Sprites/Kimber/Kimber_Idle/KimberIdle.KimberIdle" :`true` "/Game/2DSideScroller/Sprites/Astrid/Astrid_Run_Flipbook.Astrid_Run_Flipbook" :!type "PaperFlipbook Object Reference"))
    (set `self.isIdle` false))
  (`/Engine/EditorBlueprintResources/StandardMacros.CompareFloat` (.x (`MovementComponent.Velocity` (`self.CharacterMovement`)))
    (:`>`
      (`Controller.SetControlRotation` (`self.GetController`) (`KismetMathLibrary.MakeRotator` 0.0)))
    (:`<`
      (`Controller.SetControlRotation` (`self.GetController`) (`KismetMathLibrary.MakeRotator` 0.0 0.0 180.0))))
  (switch `/Game/Blueprints/Char_States` (`self.State`)
    (:`NewEnumerator0`
      (if (not (`self.isJumping`))
        (set `self.isIdle` true)
        (`PaperFlipbookComponent.SetFlipbook` (`self.Sprite`) (select `bool` (> (`KismetMathLibrary.VSize` (`KismetMathLibrary.Conv_DoubleToVector` _returnvalue_x)) 0.0) :`false` "/Game/2DSideScroller/Sprites/Kimber/Kimber_Idle/KimberIdle.KimberIdle" :`true` "/Game/2DSideScroller/Sprites/Astrid/Astrid_Run_Flipbook.Astrid_Run_Flipbook" :!type "PaperFlipbook Object Reference"))))
    (:`NewEnumerator2`
      (`PaperFlipbookComponent.SetFlipbook` (`self.Sprite`) "/Game/2DSideScroller/Sprites/Astrid/Astrid_Jump/Astrid_Jumping.Astrid_Jumping"))
    (:`NewEnumerator4`
      (`PaperFlipbookComponent.SetFlipbook` (`self.Sprite`) "/Game/2DSideScroller/Sprites/Astrid/AstridHit/Astrid_Hit1.Astrid_Hit1")
      (`KismetSystemLibrary.Delay` 1.0))
    (:`NewEnumerator7`
      (`PaperFlipbookComponent.SetFlipbook` (`self.Sprite`) "/Game/2DSideScroller/Sprites/Astrid/AstridHit/Astrid_Hit1.Astrid_Hit1"))))

(event `self.ReceiveAnyDamage`
  (params (Damage :type "Float (single-precision)") (DamageType :type "DamageType Object Reference") (InstigatedBy :type "Controller Object Reference") (DamageCauser :type "Actor Object Reference"))
  (set `self.healthperc` (+ Damage (`self.healthperc`)))
  (`self.LaunchCharacter` (`self.GetVelocity` DamageCauser)))

(event `InputTouch`
  (params (Location :type "Vector Structure") (FingerIndex :type "ETouchIndex Enum"))
  ;[1 1 1] General Animations
  (:`Pressed`
    (goto _label_2))
  (:`Released`
    (goto _label_3)))

(event `InputAxis|Move`
  (params (AxisValue :type "Float (single-precision)"))
  ;[1 1 1] Running Animation
  (`self.AddMovementInput` (`KismetMathLibrary.GetForwardVector` (struct)) AxisValue)
  (set `self.State` "NewEnumerator0"))

(event `InputAction|Special`
  (params (Key :type "Key Structure"))
  (bind _returnvalue (`self.GetControlRotation`))
  (:`Pressed`
    ;[1 1 1] Projectile on E press
    (if (not (`self.isJumping`))
      (set `self.isIdle` false)
      (set `MovementComponent.Velocity` (0.0 0.0 0.0) (`self.CharacterMovement`))
      (`PaperFlipbookComponent.SetFlipbook` (`self.Sprite`) "/Game/2DSideScroller/Sprites/Astrid/Astrid_Shoot/AstridNSpecialfast.AstridNSpecialfast")
      (`KismetSystemLibrary.Delay` 0.15)
      (set `self.isIdle` true)
      (`|SpawnActorFromClass` "/Game/Blueprints/projectile.projectile_C" (`KismetMathLibrary.MakeTransform` (+ (`self.K2_GetActorLocation`) (* (`KismetMathLibrary.GetForwardVector` _returnvalue) 25.0)) _returnvalue) "Undefined" "OverrideRootScale" null null))))

(event `InputAction|Dash`
  (params (Key :type "Key Structure"))
  (bind _returnvalue_x (`KismetMathLibrary.BreakVector` (`self.GetActorForwardVector`)))
  (bind _charactermovement (`self.CharacterMovement`))
  ;[1 1 1] Dash on Shift (In air)
  (:`Pressed`
    (if (`NavMovementComponent.IsFalling` (`self.CharacterMovement`))
      (set `MovementComponent.Velocity` (0.0 0.0 0.0) (`self.CharacterMovement`))
      (set `self.State` "NewEnumerator7")
      (set `self.isDashing` true)
      (set `CharacterMovementComponent.GroundFriction` 0.0 _charactermovement)
      (if (`NavMovementComponent.IsFalling` _charactermovement)
        (if (`self.canAirDash`)
          (if (`self.isDashing`)
            (set `MovementComponent.Velocity` (`KismetMathLibrary.MakeVector` (* _returnvalue_x (`self.dashVelocity`)) (`self.zero`) (`self.zero`)) (`self.CharacterMovement`))
            (set `CharacterMovementComponent.GravityScale` 0.0 (`self.CharacterMovement`))
            (set `self.canAirDash` false)
            (set `self.State` "NewEnumerator7")
            (`KismetSystemLibrary.Delay` 0.2)
            (set `CharacterMovementComponent.GravityScale` 3.0 (`self.CharacterMovement`))
            (set `MovementComponent.Velocity` (0.0 0.0 0.0) (`self.CharacterMovement`))
            (set `self.State` "NewEnumerator2")
            (else
              (set `CharacterMovementComponent.GroundFriction` 3.0 (`self.CharacterMovement`))))))))
  (:`Released`
    (if (`NavMovementComponent.IsFalling` (`self.CharacterMovement`))
      (set `self.State` "NewEnumerator7")
      (`PaperFlipbookComponent.SetFlipbook` (`self.Sprite`) "/Game/2DSideScroller/Sprites/Astrid/Astrid_Dash/Astrid_Air_Dodge_Dash.Astrid_Air_Dodge_Dash")
      (set `self.isDashing` false)
      (set `CharacterMovementComponent.GroundFriction` 3.0 _charactermovement))))

(event `Key|L`
  (params (Key :type "Key Structure"))
  (:`Pressed`
    (`self.K2_DestroyActor`)))

(fn `UserConstructionScript`
  (bind _charactermovement (`self.CharacterMovement`))
  (set `self.JumpMaxHoldTime` 0.2)
  (set `CharacterMovementComponent.GravityScale` 1.5 _charactermovement)
  (set `CharacterMovementComponent.GroundFriction` 3.0 _charactermovement)
  (set `CharacterMovementComponent.JumpZVelocity` 350.0 _charactermovement)
  (set `CharacterMovementComponent.AirControl` 0.3 _charactermovement)
  (set `CharacterMovementComponent.AirControlBoostMultiplier` 0.0 _charactermovement)
  (set `CharacterMovementComponent.AirControlBoostVelocityThreshold` 0.0 _charactermovement)
  (set `CharacterMovementComponent.MaxAcceleration` 2000.0 _charactermovement)
  (`PaperFlipbookComponent.SetFlipbook` (`self.Sprite`) "/Game/2DSideScroller/Sprites/Kimber/Kimber_Idle/KimberIdle.KimberIdle")
  (set `self.State` "NewEnumerator0"))