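; A projectile actor that flies straight and deals fixed damage to whatever it hits.
; The construction script turns off gravity on ProjectileMovement and sets its initial speed.
; On Hit it applies damage, hides itself, spawns a small emitter at the impact point and destroys itself after a short delay.
; An unused, disconnected sphere-trace branch that casts to Astrid1 remains in the event graph.
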(event `self.ReceiveTick`
  (params (DeltaSeconds :type "Float (single-precision)")))

(event `self.StaticMesh.OnComponentHit`
  (params (HitComponent :type "PrimitiveComponent Object Reference") (OtherActor :type "Actor Object Reference") (OtherComp :type "PrimitiveComponent Object Reference") (NormalImpulse :type "Vector Structure") (Hit :type "HitResult Structure (by ref)")))

(event `self.ReceiveHit`
  (params (MyComp :type "PrimitiveComponent Object Reference") (Other :type "Actor Object Reference") (OtherComp :type "PrimitiveComponent Object Reference") (bSelfMoved :type Boolean) (HitLocation :type "Vector Structure") (HitNormal :type "Vector Structure") (NormalImpulse :type "Vector Structure") (Hit :type "HitResult Structure (by ref)"))
  (bind (_bblockinghit _binitialoverlap _time _distance _location _impactpoint _normal _impactnormal _physmat _hitactor) (`GameplayStatics.BreakHitResult` Hit))
  (`GameplayStatics.ApplyDamage` _hitactor 10.0 null self)
  (`self.SetActorHiddenInGame` self true)
  (`GameplayStatics.SpawnEmitterAtLocation` null _location (struct) (0.1 0.1 0.1))
  (`KismetSystemLibrary.Delay` 0.2)
  (`self.K2_DestroyActor`))

(fn `UserConstructionScript`
  (bind _projectilemovement (`self.ProjectileMovement`))
  (set `ProjectileMovementComponent.ProjectileGravityScale` 0.0 _projectilemovement)
  (set `ProjectileMovementComponent.InitialSpeed` 350.0 _projectilemovement))