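; Test Paper2D player character for Astrid, a side-scroller hero with running, jumping, an air dash and a projectile special.
; Input events set a Standing/Jumping/Dashing state and flags, while a Tick update selects flipbooks and yaws the controller by horizontal velocity.
; The air dash suspends gravity for a timed horizontal burst and recharges on landing.
; The special zeroes velocity and spawns a projectile after a short animation delay.
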(event `self.ReceiveTick`
  (params (DeltaSeconds :type "Float (single-precision)"))
  (`self.UpdateAnimation1`))

(event `self.OnLanded`
  (params (Hit :type "HitResult Structure (by ref)"))
  (set `self.canAirDash` true)
  (set `self.State` "NewEnumerator0")
  (set `self.isIdle` true)
  (set `self.isJumping` false))

(event `InputAction|Jump`
  (params (Key :type "Key Structure"))
  (bind _returnvalue (`GameplayStatics.GetPlayerCharacter` 0))
  (:`Pressed`
    (bind _asastrid (cast `/Game/Blueprints/Astrid` _returnvalue))
    (`PaperFlipbookComponent.SetFlipbook` (`PaperCharacter.Sprite` _asastrid) "/Game/2DSideScroller/Sprites/Astrid/Astrid_Jump/Astrid_Jumping.Astrid_Jumping")
    (set `self.State` "NewEnumerator2"))
  (:`Released`
    (bind _asastrid_2 (cast `/Game/Blueprints/Astrid` _returnvalue))
    (`PaperFlipbookComponent.SetFlipbook` (`PaperCharacter.Sprite` _asastrid_2) "/Game/2DSideScroller/Sprites/Astrid/Astrid_Idle_Idle.Astrid_Idle_Idle")))

(event `InputAction|Jump`
  (params (Key :type "Key Structure"))
  (:`Pressed`
    (set `self.isJumping` true)
    (set `self.isIdle` false)
    (if (not (`self.isDashing`)) :!label _label
      (`self.Jump`)
      (`PaperFlipbookComponent.SetFlipbook` (`self.Sprite`) "/Game/2DSideScroller/Sprites/Astrid/Astrid_Jump/Astrid_Jumping.Astrid_Jumping")))
  (:`Released`
    (set `self.isJumping` true)
    (set `self.isIdle` false)
    (if (not (`self.isDashing`)) :!label _label_2
      (`self.StopJumping`)
      (set `self.State` "NewEnumerator0"))))

(event `UpdateAnimation1`
  (bind _returnvalue_x (`KismetMathLibrary.BreakVector` (`self.GetVelocity`)))
  (bind _returnvalue_x_2 (`KismetMathLibrary.BreakVector` (`self.GetVelocity`)))
  (if (`self.isIdle`)
    (`PaperFlipbookComponent.SetFlipbook` (`self.Sprite`) (select `bool` (> (`KismetMathLibrary.VSize` (`KismetMathLibrary.Conv_DoubleToVector` _returnvalue_x_2)) 0.0) :`false` "/Game/2DSideScroller/Sprites/Astrid/Astrid_Idle_Flipbook.Astrid_Idle_Flipbook" :`true` "/Game/2DSideScroller/Sprites/Astrid/Astrid_Run_Flipbook.Astrid_Run_Flipbook" :!type "PaperFlipbook Object Reference"))
    (set `self.isIdle` false))
  (`/Engine/EditorBlueprintResources/StandardMacros.CompareFloat` (.x (`MovementComponent.Velocity` (`self.CharacterMovement`)))
    (:`>`
      (`Controller.SetControlRotation` (`self.GetController`) (`KismetMathLibrary.MakeRotator` 0.0)))
    (:`<`
      (`Controller.SetControlRotation` (`self.GetController`) (`KismetMathLibrary.MakeRotator` 0.0 0.0 180.0))))
  (switch `/Game/Blueprints/Char_States` (`self.State`)
    (:`NewEnumerator0`
      (if (not (`self.isJumping`))
        (set `self.isIdle` true)
        (`PaperFlipbookComponent.SetFlipbook` (`self.Sprite`) (select `bool` (> (`KismetMathLibrary.VSize` (`KismetMathLibrary.Conv_DoubleToVector` _returnvalue_x)) 0.0) :`false` "/Game/2DSideScroller/Sprites/Astrid/Astrid_Idle_Flipbook.Astrid_Idle_Flipbook" :`true` "/Game/2DSideScroller/Sprites/Astrid/Astrid_Run_Flipbook.Astrid_Run_Flipbook" :!type "PaperFlipbook Object Reference"))))
    (:`NewEnumerator2`
      (`PaperFlipbookComponent.SetFlipbook` (`self.Sprite`) "/Game/2DSideScroller/Sprites/Astrid/Astrid_Jump/Astrid_Jumping.Astrid_Jumping"))
    (:`NewEnumerator7`
      (`PaperFlipbookComponent.SetFlipbook` (`self.Sprite`) "/Game/2DSideScroller/Sprites/Astrid/Astrid_Dash/Astrid_Air_Dodge_Dash.Astrid_Air_Dodge_Dash"))))

(event `InputTouch`
  (params (Location :type "Vector Structure") (FingerIndex :type "ETouchIndex Enum"))
  (:`Pressed`
    (goto _label))
  (:`Released`
    (goto _label_2)))

(event `InputAxis|MoveRight`
  (params (AxisValue :type "Float (single-precision)"))
  ;[1 1 1] Running Animation
  (`self.AddMovementInput` (`KismetMathLibrary.GetForwardVector` (struct)) AxisValue)
  (set `self.State` "NewEnumerator0"))

(event `InputAction|Special`
  (params (Key :type "Key Structure"))
  (bind _returnvalue (`self.GetControlRotation`))
  ;[1 1 1] Projectile on E press
  (:`Pressed`
    (set `self.isIdle` false)
    (set `MovementComponent.Velocity` (0.0 0.0 0.0) (`self.CharacterMovement`))
    (`PaperFlipbookComponent.SetFlipbook` (`self.Sprite`) "/Game/2DSideScroller/Sprites/Astrid/Astrid_Shoot/AstridNSpecial.AstridNSpecial")
    (`KismetSystemLibrary.Delay` 0.4)
    (set `self.isIdle` true)
    (`|SpawnActorFromClass` "/Game/2DSideScroller/projectile.projectile_C" (`KismetMathLibrary.MakeTransform` (+ (`self.K2_GetActorLocation`) (* (`KismetMathLibrary.GetForwardVector` _returnvalue) 20.0)) _returnvalue) "Undefined" "OverrideRootScale" null null)))

(event `InputAction|Dash`
  (params (Key :type "Key Structure"))
  (bind _returnvalue_x (`KismetMathLibrary.BreakVector` (`self.GetActorForwardVector`)))
  (bind _charactermovement (`self.CharacterMovement`))
  (:`Pressed`
    (if (`NavMovementComponent.IsFalling` (`self.CharacterMovement`))
      (set `MovementComponent.Velocity` (0.0 0.0 0.0) (`self.CharacterMovement`))
      (set `self.State` "NewEnumerator7")
      (`PaperFlipbookComponent.SetFlipbook` (`self.Sprite`) "/Game/2DSideScroller/Sprites/Astrid/Astrid_Dash/Astrid_Air_Dodge_Dash.Astrid_Air_Dodge_Dash")
      ;[1 1 1] Dash
      (set `self.isDashing` true)
      (set `CharacterMovementComponent.GroundFriction` 0.0 _charactermovement)
      (if (`NavMovementComponent.IsFalling` _charactermovement)
        (if (`self.canAirDash`)
          (if (`self.isDashing`)
            (set `MovementComponent.Velocity` (`KismetMathLibrary.MakeVector` (* _returnvalue_x (`self.dashVelocity`)) (`self.zero`) (`self.zero`)) (`self.CharacterMovement`))
            (set `CharacterMovementComponent.GravityScale` 0.0 (`self.CharacterMovement`))
            (set `self.canAirDash` false)
            (set `self.State` "NewEnumerator7")
            (`KismetSystemLibrary.Delay` 0.5)
            (set `CharacterMovementComponent.GravityScale` 3.0 (`self.CharacterMovement`))
            (set `MovementComponent.Velocity` (0.0 0.0 0.0) (`self.CharacterMovement`))
            (set `self.State` "NewEnumerator2")
            (else
              (set `CharacterMovementComponent.GroundFriction` 3.0 (`self.CharacterMovement`))))))))
  (:`Released`
    (if (`NavMovementComponent.IsFalling` (`self.CharacterMovement`))
      (set `self.State` "NewEnumerator7")
      (`PaperFlipbookComponent.SetFlipbook` (`self.Sprite`) "/Game/2DSideScroller/Sprites/Astrid/Astrid_Dash/Astrid_Air_Dodge_Dash.Astrid_Air_Dodge_Dash")
      (set `self.isDashing` false)
      (set `CharacterMovementComponent.GroundFriction` 3.0 _charactermovement))))

(fn `UserConstructionScript`
  (bind _charactermovement (`self.CharacterMovement`))
  (set `self.JumpMaxHoldTime` 0.2)
  (set `CharacterMovementComponent.GravityScale` 1.5 _charactermovement)
  (set `CharacterMovementComponent.GroundFriction` 3.0 _charactermovement)
  (set `CharacterMovementComponent.JumpZVelocity` 350.0 _charactermovement)
  (set `CharacterMovementComponent.AirControl` 0.3 _charactermovement)
  (set `CharacterMovementComponent.AirControlBoostMultiplier` 0.0 _charactermovement)
  (set `CharacterMovementComponent.AirControlBoostVelocityThreshold` 0.0 _charactermovement)
  (set `CharacterMovementComponent.MaxAcceleration` 2000.0 _charactermovement)
  (`PaperFlipbookComponent.SetFlipbook` (`self.Sprite`) "/Game/2DSideScroller/Sprites/Astrid/Astrid_Idle_Idle.Astrid_Idle_Idle")
  (set `self.State` "NewEnumerator0"))